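; Player actor that moves on a bounded X/Y plane via Enhanced Input, squashing along its movement axis and spawning Niagara trail puffs.
; Dash input sets CurrentSpeed, but movement reads MoveSpeed, so dashing has no effect here.
; Bullet overlaps decrement Health, destroy one cube per hit, and show the game-over widget once Health drops below zero.
; A timed shield routine exists but is never run.
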(event `self.ReceiveBeginPlay`
  (bind _asplayer_controller (cast `PlayerController` (`self.GetController`)))
  (message `EnhancedInputSubsystemInterface.AddMappingContext` (pcsubsystem `EnhancedInputLocalPlayerSubsystem` _asplayer_controller) "/Game/Preset/IMC_Main.IMC_Main" 0 (struct))
  (set `self.Health` 4))

(event `EnhancedInput|/Game/Preset/Input/IA_Dash`
  (params (ActionValue :type Boolean) (ElapsedSeconds :type "Float (double-precision)") (TriggeredSeconds :type "Float (double-precision)") (InputAction :type "InputAction Object Reference" :default "/Game/Preset/Input/IA_Dash.IA_Dash"))
  (:`Triggered`
    (set `self.CurrentSpeed` (`self.DashSpeed`)))
  (:`Completed`
    (set `self.CurrentSpeed` (`self.MoveSpeed`))))

(event `EnhancedInput|/Game/Preset/Input/IA_Move`
  (params (ActionValue :type "Vector2D Structure") (ElapsedSeconds :type "Float (double-precision)") (TriggeredSeconds :type "Float (double-precision)") (InputAction :type "InputAction Object Reference" :default "/Game/Preset/Input/IA_Move.IA_Move"))
  (bind (_returnvalue_x _returnvalue_y) (`KismetMathLibrary.BreakVector` (+ (* (`KismetMathLibrary.Normal2D` (`KismetMathLibrary.Conv_VectorToVector2D` (`KismetMathLibrary.MakeVector` ActionValue_Y ActionValue_X))) (`self.MoveSpeed`)) (`self.K2_GetActorLocation`))))
  (:`Triggered`
    (`|ExecutionSequence`
      (:`then_0`
        ;[1 1 1] Move
        (if (and (< _returnvalue_x 270.0) (> _returnvalue_x -270.0) (< _returnvalue_y 492.0) (> _returnvalue_y -492.0))
          (`self.K2_SetActorLocation` (`KismetMathLibrary.MakeVector` _returnvalue_x _returnvalue_y))
          (`|ExecutionSequence`
            (:`then_0`
              ;[1 1 1] Scale
              (if (!= (`self.Action Value Y`) 0.0)
                (`self.SetActorScale3D` (1.0 0.6 1.0))))
            (:`then_1`
              (if (!= (`self.Action Value X`) 0.0)
                (`self.SetActorScale3D` (0.6 1.0 1.0))))
            (:`then_2`
              ;[1 1 1] Particle
              (`KismetSystemLibrary.Delay` 0.05)
              (`NiagaraFunctionLibrary.SpawnSystemAtLocation` "/Game/Blueprint/NS/NS_PlayerTail.NS_PlayerTail" (`SceneComponent.K2_GetComponentLocation` (`self.Arrow`)))))))
      (:`then_1`
        (set `self.Action Value X` ActionValue_X))
      (:`then_2`
        (set `self.Action Value Y` ActionValue_Y))))
  (:`Completed`
    (`self.SetActorScale3D` (1.0 1.0 1.0))))

(event `self.Box Col.OnComponentBeginOverlap`
  (params (OverlappedComponent :type "PrimitiveComponent Object Reference") (OtherActor :type "Actor Object Reference") (OtherComp :type "PrimitiveComponent Object Reference") (OtherBodyIndex :type Integer) (bFromSweep :type Boolean) (SweepResult :type "HitResult Structure (by ref)"))
  (cast `/Game/Blueprint/BP_Bullet` OtherActor)
  (bind _output_get (set `self.Health` (- (`self.Health`) 1)))
  (`KismetSystemLibrary.PrintString` (`KismetStringLibrary.Conv_IntToString` _output_get))
  (if (< _output_get 0)
    ;[1 1 1] GameOver UI
    (bind _returnvalue (`|CreateWidget` "/Game/Blueprint/UI/BP_GameOverUI.BP_GameOverUI_C"))
    (`UserWidget.AddToViewport` _returnvalue 0)
    (else
      ;[1 1 1] Delete Cube
      (switch `int` (`self.Health`)
        (:`0`
          (`ActorComponent.K2_DestroyComponent` (`self.Cube3`)))
        (:`1`
          (`ActorComponent.K2_DestroyComponent` (`self.Cube2`)))
        (:`2`
          (`ActorComponent.K2_DestroyComponent` (`self.Cube1`)))
        (:`3`
          (`ActorComponent.K2_DestroyComponent` (`self.Cube`)))))))

(fn `UserConstructionScript`)