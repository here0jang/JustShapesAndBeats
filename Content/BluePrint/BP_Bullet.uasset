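; BP_Bullet is a short-lived bullet actor with a pulsing cube visual and no movement logic of its own.
; BeginPlay creates a dynamic fade material whose opacity a timeline drives, with a delay off the timeline's update destroying the actor seconds later.
; Tick grows the actor's scale steadily, periodically snapping it back to zero.
; Box overlap with a BP_Destroyer destroys it immediately; SetBullet is an empty stub.
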(event `self.ReceiveBeginPlay`
  (bind _returnvalue (`PrimitiveComponent.CreateDynamicMaterialInstance` (`self.Cube`) 0 "/Game/Materials/Mat_Bullet_Fade.Mat_Bullet_Fade" "None"))
  (bind _output_get (set `self.MatInstance` _returnvalue))
  (`MaterialInstanceDynamic.SetScalarParameterValue` _output_get "OpacityAmount" 2.0)
  (bind (_direction _newtrack_0) (`Timeline|Timeline`)
    (:`Update`
      (`MaterialInstanceDynamic.SetScalarParameterValue` (`self.MatInstance`) "OpacityAmount" _newtrack_0)
      (`KismetSystemLibrary.Delay` 5.0)
      (`self.K2_DestroyActor`))))

(event `self.ReceiveTick`
  (params (DeltaSeconds :type "Float (single-precision)"))
  (bind _returnvalue (* DeltaSeconds 2.0))
  (bind _output_get (set `self.CurrentTime` (+ DeltaSeconds (`self.CurrentTime`))))
  (if (> _output_get 0.8)
    (`self.SetActorScale3D` (0.0 0.0 0.0))
    (set `self.CurrentTime` 0.0)
    (else
      (`self.SetActorScale3D` (+ (`self.GetActorScale3D`) (`KismetMathLibrary.MakeVector` _returnvalue _returnvalue _returnvalue))))))

(event `self.BoxCol.OnComponentBeginOverlap`
  (params (OverlappedComponent :type "PrimitiveComponent Object Reference") (OtherActor :type "Actor Object Reference") (OtherComp :type "PrimitiveComponent Object Reference") (OtherBodyIndex :type Integer) (bFromSweep :type Boolean) (SweepResult :type "HitResult Structure (by ref)"))
  (cast `/Game/BluePrint/BP_Destroyer` OtherActor)
  (`self.K2_DestroyActor`))

(fn `SetBullet`)

(fn `UserConstructionScript`)