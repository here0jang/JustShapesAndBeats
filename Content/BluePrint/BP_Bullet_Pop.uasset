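; BP_Bullet_Pop is a bullet that travels, swells and bursts into four smaller projectiles.
; Tick moves it along negative Y until it reaches a fixed Y threshold, then accumulates time while steadily scaling the actor up.
; When the timer expires, it shrinks the sphere to zero, spawns BP_Bullet5 at four child actor positions and destroys itself.
; SetBullet and the construction script are empty.
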(event `self.ReceiveTick`
  (params (DeltaSeconds :type "Float (single-precision)"))
  (bind (_returnvalue_x _returnvalue_y) (`KismetMathLibrary.BreakVector` (`self.K2_GetActorLocation`)))
  (bind _returnvalue (* (`GameplayStatics.GetWorldDeltaSeconds`) 3.5))
  (if (> _returnvalue_y 240.0)
    (`self.K2_SetActorLocation` (+ (`self.K2_GetActorLocation`) (`KismetMathLibrary.MakeVector` 0.0 (* -160.0 (`GameplayStatics.GetWorldDeltaSeconds`)))))
    (else
      (bind _output_get (set `self.CurrentTime` (+ (`GameplayStatics.GetWorldDeltaSeconds`) (`self.CurrentTime`))))
      (if (> _output_get 0.8)
        (`SceneComponent.SetWorldScale3D` (`self.Sphere`) (0.0 0.0 0.0))
        (`|SpawnActorFromClass` "/Game/Blueprint/BP_Bullet5.BP_Bullet5_C" (`KismetMathLibrary.MakeTransform` (`SceneComponent.K2_GetComponentLocation` (`self.ChildActor`))) "Undefined" "MultiplyWithRoot" null null)
        (`|SpawnActorFromClass` "/Game/Blueprint/BP_Bullet5.BP_Bullet5_C" (`KismetMathLibrary.MakeTransform` (`SceneComponent.K2_GetComponentLocation` (`self.ChildActor1`))) "Undefined" "MultiplyWithRoot" null null)
        (`|SpawnActorFromClass` "/Game/Blueprint/BP_Bullet5.BP_Bullet5_C" (`KismetMathLibrary.MakeTransform` (`SceneComponent.K2_GetComponentLocation` (`self.ChildActor2`))) "Undefined" "MultiplyWithRoot" null null)
        (`|SpawnActorFromClass` "/Game/Blueprint/BP_Bullet5.BP_Bullet5_C" (`KismetMathLibrary.MakeTransform` (`SceneComponent.K2_GetComponentLocation` (`self.ChildActor3`))) "Undefined" "MultiplyWithRoot" null null)
        (`self.K2_DestroyActor`)
        (else
          (`self.SetActorScale3D` (+ (`self.GetActorScale3D`) (`KismetMathLibrary.MakeVector` _returnvalue _returnvalue _returnvalue))))))))

(fn `SetBullet`)

(fn `UserConstructionScript`)