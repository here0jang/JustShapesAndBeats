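; BP_Bullet5 is a bullet actor that travels in a straight line along its negative right vector.
; Tick moves it a fixed distance each frame with no sweep or delta-time scaling, so its speed depends on frame rate.
; An unconnected branch holds unused Y-threshold, timer, scaling and NS_PlayerTail Niagara spawn logic, and SetBullet is an empty stub.
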(event `self.ReceiveBeginPlay`)

(event `self.ReceiveTick`
  (params (DeltaSeconds :type "Float (single-precision)"))
  (`self.K2_SetActorLocation` (+ (* (`self.GetActorRightVector`) -4.0) (`self.K2_GetActorLocation`))))

(fn `SetBullet`)

(fn `UserConstructionScript`)