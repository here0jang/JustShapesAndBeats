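; BP_Bullet4 is a bullet actor whose visible behavior is a repeating grow-and-reset scale pulse.
; Tick accumulates elapsed time and grows the actor's scale uniformly at a constant rate, snapping it back to zero and restarting the timer after a short fixed interval.
; SetBullet, BeginPlay and the construction script are empty, and a leftover Delay node is unconnected.
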(event `self.ReceiveBeginPlay`)

(event `self.ReceiveTick`
  (params (DeltaSeconds :type "Float (single-precision)"))
  (bind _returnvalue (* DeltaSeconds 2.0))
  (bind _output_get (set `self.CurrentTime` (+ DeltaSeconds (`self.CurrentTime`))))
  (if (> _output_get 0.8)
    (`self.SetActorScale3D` (0.0 0.0 0.0))
    (set `self.CurrentTime` 0.0)
    (else
      (`self.SetActorScale3D` (+ (`self.GetActorScale3D`) (`KismetMathLibrary.MakeVector` _returnvalue _returnvalue _returnvalue))))))

(fn `SetBullet`)

(fn `UserConstructionScript`)