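; Scripted bullet spawner that plays a fixed, timed pattern of bullet waves from BeginPlay.
; A long chain of Delay and nested Sequence nodes spawns actors at hard-coded locations, with branches offsetting overlapping shots.
; Waves progress from small cubes through big cubes to rows of arrows along one Y edge, then pop and arrow Reverse variants, with the arrows coming from the opposite edge.
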(event `self.ReceiveBeginPlay`
  ;[1 1 1] Small Cube
  (`|ExecutionSequence`
    (:`then_0`
      (`|SpawnActorFromClass` "/Game/Blueprint/BP_Bullet.BP_Bullet_C" (`KismetMathLibrary.MakeTransform` (-140.0 -240.0 15.0) (struct) (0.1 0.1 0.1)) "Undefined" "MultiplyWithRoot" null null)
      (`KismetSystemLibrary.Delay` 0.4 :!label _label)
      (`|ExecutionSequence`
        (:`then_0`
          (`|SpawnActorFromClass` "/Game/Blueprint/BP_Bullet.BP_Bullet_C" (`KismetMathLibrary.MakeTransform` (60.0 380.0 15.0) (struct) (0.1 0.1 0.1)) "Undefined" "MultiplyWithRoot" null null))
        (:`then_1`
          (`|SpawnActorFromClass` "/Game/Blueprint/BP_Bullet.BP_Bullet_C" (`KismetMathLibrary.MakeTransform` (-20.0 440.0 15.0) (struct) (0.1 0.1 0.1)) "Undefined" "MultiplyWithRoot" null null)
          (`KismetSystemLibrary.Delay` 0.4)
          (`|SpawnActorFromClass` "/Game/Blueprint/BP_Bullet.BP_Bullet_C" (`KismetMathLibrary.MakeTransform` (-180.0 440.0 15.0) (struct) (0.1 0.1 0.1)) "Undefined" "MultiplyWithRoot" null null)
          ;[1 1 1] Comment
          ;;[1 1 1] Big Cube
          (`KismetSystemLibrary.Delay` 4.2)
          (bind _returnvalue (`|SpawnActorFromClass` "/Game/Blueprint/BP_BUllet_BigCube.BP_BUllet_BigCube_C" (`KismetMathLibrary.MakeTransform` (-200.0 -175.0 15.0)) "Undefined" "MultiplyWithRoot" null null))
          (`KismetSystemLibrary.Delay` 0.4)
          (`|ExecutionSequence`
            (:`then_0`
              (bind _returnvalue_2 (`|SpawnActorFromClass` "/Game/Blueprint/BP_BUllet_BigCube.BP_BUllet_BigCube_C" (`KismetMathLibrary.MakeTransform` (0.0 -460.0 15.0)) "Undefined" "MultiplyWithRoot" null null))
              (`KismetSystemLibrary.Delay` 0.4)
              (`|ExecutionSequence`
                (:`then_0`
                  ;;[1 1 1] Big Cube2
                  (bind _returnvalue_3 (`|SpawnActorFromClass` "/Game/Blueprint/BP_BUllet_BigCube.BP_BUllet_BigCube_C" (`KismetMathLibrary.MakeTransform` (-200.0 -460.0 15.0)) "Undefined" "MultiplyWithRoot" null null)))
                (:`then_1`
                  (bind _returnvalue_4 (`|SpawnActorFromClass` "/Game/Blueprint/BP_BUllet_BigCube.BP_BUllet_BigCube_C" (`KismetMathLibrary.MakeTransform` (-100.0 -280.0 15.0)) "Undefined" "MultiplyWithRoot" null null)))
                (:`then_2`
                  (bind _returnvalue_5 (`|SpawnActorFromClass` "/Game/Blueprint/BP_BUllet_BigCube.BP_BUllet_BigCube_C" (`KismetMathLibrary.MakeTransform` (-100.0 50.0 15.0)) "Undefined" "MultiplyWithRoot" null null))
                  (`KismetSystemLibrary.Delay` 0.4)
                  (`|ExecutionSequence`
                    (:`then_0`
                      ;;[1 1 1] Big Cube3
                      (bind _returnvalue_6 (`|SpawnActorFromClass` "/Game/Blueprint/BP_BUllet_BigCube.BP_BUllet_BigCube_C" (`KismetMathLibrary.MakeTransform` (-10.0 230.0 15.0)) "Undefined" "MultiplyWithRoot" null null))
                      (`KismetSystemLibrary.Delay` 0.4)
                      (`|ExecutionSequence`
                        (:`then_0`
                          ;;[1 1 1] Big Cube3
                          (bind _returnvalue_7 (`|SpawnActorFromClass` "/Game/Blueprint/BP_BUllet_BigCube.BP_BUllet_BigCube_C" (`KismetMathLibrary.MakeTransform` (85.0 325.0 15.0)) "Undefined" "MultiplyWithRoot" null null))
                          (`KismetSystemLibrary.Delay` 0.4)
                          (`|ExecutionSequence`
                            (:`then_0`
                              ;;[1 1 1] Comment
                              (bind _returnvalue_8 (`|SpawnActorFromClass` "/Game/Blueprint/BP_BUllet_BigCube.BP_BUllet_BigCube_C" (`KismetMathLibrary.MakeTransform` (-10.0 420.0 15.0)) "Undefined" "MultiplyWithRoot" null null))
                              (`KismetSystemLibrary.Delay` 5.2)
                              (`|ExecutionSequence`
                                (:`then_0`
                                  ;[1 1 1] Comment
                                  (`|SpawnActorFromClass` "/Game/Blueprint/BP_Bullet_Pop.BP_Bullet_Pop_C" (`KismetMathLibrary.MakeTransform` (220.0 550.0 15.0)) "Undefined" "MultiplyWithRoot" null null)
                                  (`KismetSystemLibrary.Delay` 2.4)
                                  (`|SpawnActorFromClass` "/Game/Blueprint/BP_Bullet_Arrow.BP_Bullet_Arrow_C" (`KismetMathLibrary.MakeTransform` (-100.0 630.0 15.0)) "Undefined" "MultiplyWithRoot" null null)
                                  (`KismetSystemLibrary.Delay` 0.4)
                                  (`|ExecutionSequence`
                                    (:`then_0`
                                      (`KismetSystemLibrary.Delay` 0.2)
                                      (`|SpawnActorFromClass` "/Game/Blueprint/BP_Bullet_Arrow.BP_Bullet_Arrow_C" (`KismetMathLibrary.MakeTransform` (200.0 630.0 15.0)) "Undefined" "MultiplyWithRoot" null null))
                                    (:`then_1`
                                      (`|SpawnActorFromClass` "/Game/Blueprint/BP_Bullet_Arrow.BP_Bullet_Arrow_C" (`KismetMathLibrary.MakeTransform` (-140.0 630.0 15.0)) "Undefined" "MultiplyWithRoot" null null)
                                      (`KismetSystemLibrary.Delay` 0.4)
                                      (`|ExecutionSequence`
                                        (:`then_0`
                                          (`KismetSystemLibrary.Delay` 0.2)
                                          (`|SpawnActorFromClass` "/Game/Blueprint/BP_Bullet_Arrow.BP_Bullet_Arrow_C" (`KismetMathLibrary.MakeTransform` (-180.0 630.0 15.0)) "Undefined" "MultiplyWithRoot" null null)
                                          (`KismetSystemLibrary.Delay` 0.4)
                                          (`|SpawnActorFromClass` "/Game/Blueprint/BP_Bullet_Arrow.BP_Bullet_Arrow_C" (`KismetMathLibrary.MakeTransform` (-20.0 630.0 15.0)) "Undefined" "MultiplyWithRoot" null null)
                                          (`KismetSystemLibrary.Delay` 0.4)
                                          (`|SpawnActorFromClass` "/Game/Blueprint/BP_Bullet_Arrow.BP_Bullet_Arrow_C" (`KismetMathLibrary.MakeTransform` (-80.0 630.0 15.0)) "Undefined" "MultiplyWithRoot" null null)
                                          (`KismetSystemLibrary.Delay` 0.4)
                                          (`|SpawnActorFromClass` "/Game/Blueprint/BP_Bullet_Arrow.BP_Bullet_Arrow_C" (`KismetMathLibrary.MakeTransform` (260.0 630.0 15.0)) "Undefined" "MultiplyWithRoot" null null)
                                          (`KismetSystemLibrary.Delay` 0.4)
                                          (`|SpawnActorFromClass` "/Game/Blueprint/BP_Bullet_Arrow.BP_Bullet_Arrow_C" (`KismetMathLibrary.MakeTransform` (220.0 630.0 15.0)) "Undefined" "MultiplyWithRoot" null null)
                                          (`KismetSystemLibrary.Delay` 0.4)
                                          (`|SpawnActorFromClass` "/Game/Blueprint/BP_Bullet_Arrow.BP_Bullet_Arrow_C" (`KismetMathLibrary.MakeTransform` (0.0 630.0 15.0)) "Undefined" "MultiplyWithRoot" null null)
                                          (`|ExecutionSequence`
                                            (:`then_0`
                                              (`KismetSystemLibrary.Delay` 0.4)
                                              (`|SpawnActorFromClass` "/Game/Blueprint/BP_Bullet_Arrow.BP_Bullet_Arrow_C" (`KismetMathLibrary.MakeTransform` (260.0 630.0 15.0)) "Undefined" "MultiplyWithRoot" null null))
                                            (:`then_1`
                                              (`KismetSystemLibrary.Delay` 0.2)
                                              (`|SpawnActorFromClass` "/Game/Blueprint/BP_Bullet_Arrow.BP_Bullet_Arrow_C" (`KismetMathLibrary.MakeTransform` (-220.0 630.0 15.0)) "Undefined" "MultiplyWithRoot" null null)
                                              (`KismetSystemLibrary.Delay` 0.4)
                                              (`|SpawnActorFromClass` "/Game/Blueprint/BP_Bullet_Arrow.BP_Bullet_Arrow_C" (`KismetMathLibrary.MakeTransform` (-180.0 630.0 15.0)) "Undefined" "MultiplyWithRoot" null null)
                                              (`KismetSystemLibrary.Delay` 0.4)
                                              (`|SpawnActorFromClass` "/Game/Blueprint/BP_Bullet_Arrow.BP_Bullet_Arrow_C" (`KismetMathLibrary.MakeTransform` (-100.0 630.0 15.0)) "Undefined" "MultiplyWithRoot" null null)
                                              (`KismetSystemLibrary.Delay` 0.4)
                                              (`|ExecutionSequence`
                                                (:`then_0`
                                                  (`KismetSystemLibrary.Delay` 0.2)
                                                  (`|SpawnActorFromClass` "/Game/Blueprint/BP_Bullet_Arrow.BP_Bullet_Arrow_C" (`KismetMathLibrary.MakeTransform` (200.0 630.0 15.0)) "Undefined" "MultiplyWithRoot" null null))
                                                (:`then_1`
                                                  (`|SpawnActorFromClass` "/Game/Blueprint/BP_Bullet_Arrow.BP_Bullet_Arrow_C" (`KismetMathLibrary.MakeTransform` (-140.0 630.0 15.0)) "Undefined" "MultiplyWithRoot" null null)
                                                  (`KismetSystemLibrary.Delay` 0.4)
                                                  (`|ExecutionSequence`
                                                    (:`then_0`
                                                      (`KismetSystemLibrary.Delay` 0.2)
                                                      (`|SpawnActorFromClass` "/Game/Blueprint/BP_Bullet_Arrow.BP_Bullet_Arrow_C" (`KismetMathLibrary.MakeTransform` (-180.0 630.0 15.0)) "Undefined" "MultiplyWithRoot" null null)
                                                      (`KismetSystemLibrary.Delay` 0.4)
                                                      (`|SpawnActorFromClass` "/Game/Blueprint/BP_Bullet_Arrow.BP_Bullet_Arrow_C" (`KismetMathLibrary.MakeTransform` (-20.0 630.0 15.0)) "Undefined" "MultiplyWithRoot" null null)
                                                      (`KismetSystemLibrary.Delay` 0.4)
                                                      (`|SpawnActorFromClass` "/Game/Blueprint/BP_Bullet_Arrow.BP_Bullet_Arrow_C" (`KismetMathLibrary.MakeTransform` (-80.0 630.0 15.0)) "Undefined" "MultiplyWithRoot" null null)
                                                      (`KismetSystemLibrary.Delay` 0.4)
                                                      (`|ExecutionSequence`
                                                        (:`then_0`
                                                          (`KismetSystemLibrary.Delay` 0.2)
                                                          (`|SpawnActorFromClass` "/Game/Blueprint/BP_Bullet_Arrow.BP_Bullet_Arrow_C" (`KismetMathLibrary.MakeTransform` (200.0 630.0 15.0)) "Undefined" "MultiplyWithRoot" null null))
                                                        (:`then_1`
                                                          (`|SpawnActorFromClass` "/Game/Blueprint/BP_Bullet_Arrow.BP_Bullet_Arrow_C" (`KismetMathLibrary.MakeTransform` (-140.0 630.0 15.0)) "Undefined" "MultiplyWithRoot" null null)
                                                          (`KismetSystemLibrary.Delay` 0.4)
                                                          (`|ExecutionSequence`
                                                            (:`then_0`
                                                              (`KismetSystemLibrary.Delay` 0.2)
                                                              (`|SpawnActorFromClass` "/Game/Blueprint/BP_Bullet_Arrow.BP_Bullet_Arrow_C" (`KismetMathLibrary.MakeTransform` (-180.0 630.0 15.0)) "Undefined" "MultiplyWithRoot" null null)
                                                              (`KismetSystemLibrary.Delay` 0.4)
                                                              (`|SpawnActorFromClass` "/Game/Blueprint/BP_Bullet_Arrow.BP_Bullet_Arrow_C" (`KismetMathLibrary.MakeTransform` (-20.0 630.0 15.0)) "Undefined" "MultiplyWithRoot" null null)
                                                              (`KismetSystemLibrary.Delay` 0.4)
                                                              (`|SpawnActorFromClass` "/Game/Blueprint/BP_Bullet_Arrow.BP_Bullet_Arrow_C" (`KismetMathLibrary.MakeTransform` (-80.0 630.0 15.0)) "Undefined" "MultiplyWithRoot" null null)
                                                              (`KismetSystemLibrary.Delay` 0.4)
                                                              (`|ExecutionSequence`
                                                                (:`then_0`
                                                                  (`KismetSystemLibrary.Delay` 0.2)
                                                                  (`|SpawnActorFromClass` "/Game/Blueprint/BP_Bullet_Arrow.BP_Bullet_Arrow_C" (`KismetMathLibrary.MakeTransform` (200.0 630.0 15.0)) "Undefined" "MultiplyWithRoot" null null))
                                                                (:`then_1`
                                                                  (`|SpawnActorFromClass` "/Game/Blueprint/BP_Bullet_Arrow.BP_Bullet_Arrow_C" (`KismetMathLibrary.MakeTransform` (-140.0 630.0 15.0)) "Undefined" "MultiplyWithRoot" null null)
                                                                  (`KismetSystemLibrary.Delay` 0.4)
                                                                  (`|ExecutionSequence`
                                                                    (:`then_0`
                                                                      (`KismetSystemLibrary.Delay` 0.2)
                                                                      (`|SpawnActorFromClass` "/Game/Blueprint/BP_Bullet_Arrow.BP_Bullet_Arrow_C" (`KismetMathLibrary.MakeTransform` (-180.0 630.0 15.0)) "Undefined" "MultiplyWithRoot" null null)
                                                                      (`KismetSystemLibrary.Delay` 0.4)
                                                                      (`|SpawnActorFromClass` "/Game/Blueprint/BP_Bullet_Arrow.BP_Bullet_Arrow_C" (`KismetMathLibrary.MakeTransform` (-20.0 630.0 15.0)) "Undefined" "MultiplyWithRoot" null null)
                                                                      (`KismetSystemLibrary.Delay` 0.4)
                                                                      (`|SpawnActorFromClass` "/Game/Blueprint/BP_Bullet_Arrow.BP_Bullet_Arrow_C" (`KismetMathLibrary.MakeTransform` (-80.0 630.0 15.0)) "Undefined" "MultiplyWithRoot" null null)
                                                                      (`KismetSystemLibrary.Delay` 2.0)
                                                                      (`|ExecutionSequence`
                                                                        (:`then_0`
                                                                          ;[1 1 1] Comment
                                                                          (`|SpawnActorFromClass` "/Game/Blueprint/BP_Bullet_Pop_Reverse.BP_Bullet_Pop_Reverse_C" (`KismetMathLibrary.MakeTransform` (220.0 -240.0 15.0)) "Undefined" "MultiplyWithRoot" null null)
                                                                          (`KismetSystemLibrary.Delay` 2.4)
                                                                          ;[1 1 1] Comment
                                                                          (`|SpawnActorFromClass` "/Game/Blueprint/BP_Bullet_Arrow_Reverse.BP_Bullet_Arrow_Reverse_C" (`KismetMathLibrary.MakeTransform` (-100.0 -630.0 15.0)) "Undefined" "MultiplyWithRoot" null null)
                                                                          (`KismetSystemLibrary.Delay` 0.4)
                                                                          (`|ExecutionSequence`
                                                                            (:`then_0`
                                                                              (`KismetSystemLibrary.Delay` 0.2)
                                                                              (`|SpawnActorFromClass` "/Game/Blueprint/BP_Bullet_Arrow_Reverse.BP_Bullet_Arrow_Reverse_C" (`KismetMathLibrary.MakeTransform` (200.0 -630.0 15.0)) "Undefined" "MultiplyWithRoot" null null)
                                                                              (`KismetSystemLibrary.Delay` 0.4)
                                                                              (`|ExecutionSequence`
                                                                                (:`then_0`
                                                                                  (`KismetSystemLibrary.Delay` 0.2)
                                                                                  (`|SpawnActorFromClass` "/Game/Blueprint/BP_Bullet_Arrow_Reverse.BP_Bullet_Arrow_Reverse_C" (`KismetMathLibrary.MakeTransform` (-180.0 -630.0 15.0)) "Undefined" "MultiplyWithRoot" null null)
                                                                                  (`KismetSystemLibrary.Delay` 0.4)
                                                                                  (`|SpawnActorFromClass` "/Game/Blueprint/BP_Bullet_Arrow_Reverse.BP_Bullet_Arrow_Reverse_C" (`KismetMathLibrary.MakeTransform` (-20.0 -630.0 15.0)) "Undefined" "MultiplyWithRoot" null null)
                                                                                  (`KismetSystemLibrary.Delay` 0.4)
                                                                                  (`|SpawnActorFromClass` "/Game/Blueprint/BP_Bullet_Arrow_Reverse.BP_Bullet_Arrow_Reverse_C" (`KismetMathLibrary.MakeTransform` (-80.0 -630.0 15.0)) "Undefined" "MultiplyWithRoot" null null)
                                                                                  (`KismetSystemLibrary.Delay` 0.4)
                                                                                  (`|SpawnActorFromClass` "/Game/Blueprint/BP_Bullet_Arrow_Reverse.BP_Bullet_Arrow_Reverse_C" (`KismetMathLibrary.MakeTransform` (260.0 -630.0 15.0)) "Undefined" "MultiplyWithRoot" null null)
                                                                                  (`KismetSystemLibrary.Delay` 0.4)
                                                                                  (`|SpawnActorFromClass` "/Game/Blueprint/BP_Bullet_Arrow_Reverse.BP_Bullet_Arrow_Reverse_C" (`KismetMathLibrary.MakeTransform` (220.0 -630.0 15.0)) "Undefined" "MultiplyWithRoot" null null)
                                                                                  (`KismetSystemLibrary.Delay` 0.4)
                                                                                  (`|SpawnActorFromClass` "/Game/Blueprint/BP_Bullet_Arrow_Reverse.BP_Bullet_Arrow_Reverse_C" (`KismetMathLibrary.MakeTransform` (0.0 -630.0 15.0)) "Undefined" "MultiplyWithRoot" null null)
                                                                                  (`|ExecutionSequence`
                                                                                    (:`then_0`
                                                                                      (`KismetSystemLibrary.Delay` 0.4)
                                                                                      (`|SpawnActorFromClass` "/Game/Blueprint/BP_Bullet_Arrow_Reverse.BP_Bullet_Arrow_Reverse_C" (`KismetMathLibrary.MakeTransform` (260.0 -630.0 15.0)) "Undefined" "MultiplyWithRoot" null null))
                                                                                    (:`then_1`
                                                                                      (`KismetSystemLibrary.Delay` 0.2)
                                                                                      (`|SpawnActorFromClass` "/Game/Blueprint/BP_Bullet_Arrow_Reverse.BP_Bullet_Arrow_Reverse_C" (`KismetMathLibrary.MakeTransform` (-220.0 -630.0 15.0)) "Undefined" "MultiplyWithRoot" null null)
                                                                                      (`KismetSystemLibrary.Delay` 0.4)
                                                                                      (`|SpawnActorFromClass` "/Game/Blueprint/BP_Bullet_Arrow_Reverse.BP_Bullet_Arrow_Reverse_C" (`KismetMathLibrary.MakeTransform` (-180.0 -630.0 15.0)) "Undefined" "MultiplyWithRoot" null null)
                                                                                      (`KismetSystemLibrary.Delay` 0.4)
                                                                                      (`|SpawnActorFromClass` "/Game/Blueprint/BP_Bullet_Arrow_Reverse.BP_Bullet_Arrow_Reverse_C" (`KismetMathLibrary.MakeTransform` (-100.0 -630.0 15.0)) "Undefined" "MultiplyWithRoot" null null)
                                                                                      (`KismetSystemLibrary.Delay` 0.4)
                                                                                      (`|ExecutionSequence`
                                                                                        (:`then_0`
                                                                                          (`KismetSystemLibrary.Delay` 0.4)
                                                                                          (`|SpawnActorFromClass` "/Game/Blueprint/BP_Bullet_Arrow_Reverse.BP_Bullet_Arrow_Reverse_C" (`KismetMathLibrary.MakeTransform` (260.0 -630.0 15.0)) "Undefined" "MultiplyWithRoot" null null))
                                                                                        (:`then_1`
                                                                                          (`KismetSystemLibrary.Delay` 0.2)
                                                                                          (`|SpawnActorFromClass` "/Game/Blueprint/BP_Bullet_Arrow_Reverse.BP_Bullet_Arrow_Reverse_C" (`KismetMathLibrary.MakeTransform` (-220.0 -630.0 15.0)) "Undefined" "MultiplyWithRoot" null null)
                                                                                          (`KismetSystemLibrary.Delay` 0.4)
                                                                                          (`|SpawnActorFromClass` "/Game/Blueprint/BP_Bullet_Arrow_Reverse.BP_Bullet_Arrow_Reverse_C" (`KismetMathLibrary.MakeTransform` (-180.0 -630.0 15.0)) "Undefined" "MultiplyWithRoot" null null)
                                                                                          (`KismetSystemLibrary.Delay` 0.4)
                                                                                          (`|SpawnActorFromClass` "/Game/Blueprint/BP_Bullet_Arrow_Reverse.BP_Bullet_Arrow_Reverse_C" (`KismetMathLibrary.MakeTransform` (-100.0 -630.0 15.0)) "Undefined" "MultiplyWithRoot" null null)
                                                                                          (`KismetSystemLibrary.Delay` 0.4)
                                                                                          (`|ExecutionSequence`
                                                                                            (:`then_0`
                                                                                              (`KismetSystemLibrary.Delay` 0.4)
                                                                                              (`|SpawnActorFromClass` "/Game/Blueprint/BP_Bullet_Arrow_Reverse.BP_Bullet_Arrow_Reverse_C" (`KismetMathLibrary.MakeTransform` (260.0 -630.0 15.0)) "Undefined" "MultiplyWithRoot" null null))
                                                                                            (:`then_1`
                                                                                              (`KismetSystemLibrary.Delay` 0.2)
                                                                                              (`|SpawnActorFromClass` "/Game/Blueprint/BP_Bullet_Arrow_Reverse.BP_Bullet_Arrow_Reverse_C" (`KismetMathLibrary.MakeTransform` (-220.0 -630.0 15.0)) "Undefined" "MultiplyWithRoot" null null)
                                                                                              (`KismetSystemLibrary.Delay` 0.4)
                                                                                              (`|SpawnActorFromClass` "/Game/Blueprint/BP_Bullet_Arrow_Reverse.BP_Bullet_Arrow_Reverse_C" (`KismetMathLibrary.MakeTransform` (-180.0 -630.0 15.0)) "Undefined" "MultiplyWithRoot" null null)
                                                                                              (`KismetSystemLibrary.Delay` 0.4)
                                                                                              (`|SpawnActorFromClass` "/Game/Blueprint/BP_Bullet_Arrow_Reverse.BP_Bullet_Arrow_Reverse_C" (`KismetMathLibrary.MakeTransform` (-100.0 -630.0 15.0)) "Undefined" "MultiplyWithRoot" null null)
                                                                                              (`KismetSystemLibrary.Delay` 0.4)
                                                                                              (`|ExecutionSequence`
                                                                                                (:`then_0`
                                                                                                  (`KismetSystemLibrary.Delay` 0.4)
                                                                                                  (`|SpawnActorFromClass` "/Game/Blueprint/BP_Bullet_Arrow_Reverse.BP_Bullet_Arrow_Reverse_C" (`KismetMathLibrary.MakeTransform` (260.0 -630.0 15.0)) "Undefined" "MultiplyWithRoot" null null))
                                                                                                (:`then_1`
                                                                                                  (`KismetSystemLibrary.Delay` 0.2)
                                                                                                  (`|SpawnActorFromClass` "/Game/Blueprint/BP_Bullet_Arrow_Reverse.BP_Bullet_Arrow_Reverse_C" (`KismetMathLibrary.MakeTransform` (-220.0 -630.0 15.0)) "Undefined" "MultiplyWithRoot" null null)
                                                                                                  (`KismetSystemLibrary.Delay` 0.4)
                                                                                                  (`|SpawnActorFromClass` "/Game/Blueprint/BP_Bullet_Arrow_Reverse.BP_Bullet_Arrow_Reverse_C" (`KismetMathLibrary.MakeTransform` (-180.0 -630.0 15.0)) "Undefined" "MultiplyWithRoot" null null)
                                                                                                  (`KismetSystemLibrary.Delay` 0.4)
                                                                                                  (`|SpawnActorFromClass` "/Game/Blueprint/BP_Bullet_Arrow_Reverse.BP_Bullet_Arrow_Reverse_C" (`KismetMathLibrary.MakeTransform` (-100.0 -630.0 15.0)) "Undefined" "MultiplyWithRoot" null null)
                                                                                                  (`KismetSystemLibrary.Delay` 0.4)
                                                                                                  (`|ExecutionSequence`
                                                                                                    (:`then_0`
                                                                                                      (`KismetSystemLibrary.Delay` 0.4)
                                                                                                      (`|SpawnActorFromClass` "/Game/Blueprint/BP_Bullet_Arrow_Reverse.BP_Bullet_Arrow_Reverse_C" (`KismetMathLibrary.MakeTransform` (260.0 -630.0 15.0)) "Undefined" "MultiplyWithRoot" null null))
                                                                                                    (:`then_1`
                                                                                                      (`KismetSystemLibrary.Delay` 0.2)
                                                                                                      (`|SpawnActorFromClass` "/Game/Blueprint/BP_Bullet_Arrow_Reverse.BP_Bullet_Arrow_Reverse_C" (`KismetMathLibrary.MakeTransform` (-220.0 -630.0 15.0)) "Undefined" "MultiplyWithRoot" null null)
                                                                                                      (`KismetSystemLibrary.Delay` 0.4)
                                                                                                      (`|SpawnActorFromClass` "/Game/Blueprint/BP_Bullet_Arrow_Reverse.BP_Bullet_Arrow_Reverse_C" (`KismetMathLibrary.MakeTransform` (-180.0 -630.0 15.0)) "Undefined" "MultiplyWithRoot" null null)
                                                                                                      (`KismetSystemLibrary.Delay` 0.4)
                                                                                                      (`|SpawnActorFromClass` "/Game/Blueprint/BP_Bullet_Arrow_Reverse.BP_Bullet_Arrow_Reverse_C" (`KismetMathLibrary.MakeTransform` (-100.0 -630.0 15.0)) "Undefined" "MultiplyWithRoot" null null)
                                                                                                      (`KismetSystemLibrary.Delay` 0.4)
                                                                                                      (`|ExecutionSequence`
                                                                                                        (:`then_0`
                                                                                                          (`KismetSystemLibrary.Delay` 0.4)
                                                                                                          (`|SpawnActorFromClass` "/Game/Blueprint/BP_Bullet_Arrow_Reverse.BP_Bullet_Arrow_Reverse_C" (`KismetMathLibrary.MakeTransform` (260.0 -630.0 15.0)) "Undefined" "MultiplyWithRoot" null null))
                                                                                                        (:`then_1`
                                                                                                          (`KismetSystemLibrary.Delay` 0.2)
                                                                                                          (`|SpawnActorFromClass` "/Game/Blueprint/BP_Bullet_Arrow_Reverse.BP_Bullet_Arrow_Reverse_C" (`KismetMathLibrary.MakeTransform` (-220.0 -630.0 15.0)) "Undefined" "MultiplyWithRoot" null null)
                                                                                                          (`KismetSystemLibrary.Delay` 0.4)
                                                                                                          (`|SpawnActorFromClass` "/Game/Blueprint/BP_Bullet_Arrow_Reverse.BP_Bullet_Arrow_Reverse_C" (`KismetMathLibrary.MakeTransform` (-180.0 -630.0 15.0)) "Undefined" "MultiplyWithRoot" null null)
                                                                                                          (`KismetSystemLibrary.Delay` 0.4)
                                                                                                          (`|SpawnActorFromClass` "/Game/Blueprint/BP_Bullet_Arrow_Reverse.BP_Bullet_Arrow_Reverse_C" (`KismetMathLibrary.MakeTransform` (-100.0 -630.0 15.0)) "Undefined" "MultiplyWithRoot" null null)
                                                                                                          (`KismetSystemLibrary.Delay` 0.4)
                                                                                                          (`|ExecutionSequence`
                                                                                                            (:`then_0`
                                                                                                              (`KismetSystemLibrary.Delay` 0.4)
                                                                                                              (`|SpawnActorFromClass` "/Game/Blueprint/BP_Bullet_Arrow_Reverse.BP_Bullet_Arrow_Reverse_C" (`KismetMathLibrary.MakeTransform` (260.0 -630.0 15.0)) "Undefined" "MultiplyWithRoot" null null))
                                                                                                            (:`then_1`
                                                                                                              (`KismetSystemLibrary.Delay` 0.2)
                                                                                                              (`|SpawnActorFromClass` "/Game/Blueprint/BP_Bullet_Arrow_Reverse.BP_Bullet_Arrow_Reverse_C" (`KismetMathLibrary.MakeTransform` (-220.0 -630.0 15.0)) "Undefined" "MultiplyWithRoot" null null)
                                                                                                              (`KismetSystemLibrary.Delay` 0.4)
                                                                                                              (`|SpawnActorFromClass` "/Game/Blueprint/BP_Bullet_Arrow_Reverse.BP_Bullet_Arrow_Reverse_C" (`KismetMathLibrary.MakeTransform` (-180.0 -630.0 15.0)) "Undefined" "MultiplyWithRoot" null null)
                                                                                                              (`KismetSystemLibrary.Delay` 0.4)
                                                                                                              (`|SpawnActorFromClass` "/Game/Blueprint/BP_Bullet_Arrow_Reverse.BP_Bullet_Arrow_Reverse_C" (`KismetMathLibrary.MakeTransform` (-100.0 -630.0 15.0)) "Undefined" "MultiplyWithRoot" null null)
                                                                                                              (`KismetSystemLibrary.Delay` 0.4)
                                                                                                              (`|ExecutionSequence`
                                                                                                                (:`then_0`
                                                                                                                  (`KismetSystemLibrary.Delay` 0.4)
                                                                                                                  (`|SpawnActorFromClass` "/Game/Blueprint/BP_Bullet_Arrow_Reverse.BP_Bullet_Arrow_Reverse_C" (`KismetMathLibrary.MakeTransform` (260.0 -630.0 15.0)) "Undefined" "MultiplyWithRoot" null null))
                                                                                                                (:`then_1`
                                                                                                                  (`KismetSystemLibrary.Delay` 0.2)
                                                                                                                  (`|SpawnActorFromClass` "/Game/Blueprint/BP_Bullet_Arrow_Reverse.BP_Bullet_Arrow_Reverse_C" (`KismetMathLibrary.MakeTransform` (-220.0 -630.0 15.0)) "Undefined" "MultiplyWithRoot" null null)
                                                                                                                  (`KismetSystemLibrary.Delay` 0.4)
                                                                                                                  (`|SpawnActorFromClass` "/Game/Blueprint/BP_Bullet_Arrow_Reverse.BP_Bullet_Arrow_Reverse_C" (`KismetMathLibrary.MakeTransform` (-180.0 -630.0 15.0)) "Undefined" "MultiplyWithRoot" null null)
                                                                                                                  (`KismetSystemLibrary.Delay` 0.4)
                                                                                                                  (`|SpawnActorFromClass` "/Game/Blueprint/BP_Bullet_Arrow_Reverse.BP_Bullet_Arrow_Reverse_C" (`KismetMathLibrary.MakeTransform` (-100.0 -630.0 15.0)) "Undefined" "MultiplyWithRoot" null null)
                                                                                                                  (`KismetSystemLibrary.Delay` 0.4)
                                                                                                                  (`|ExecutionSequence`
                                                                                                                    (:`then_0`
                                                                                                                      (`KismetSystemLibrary.Delay` 0.4)
                                                                                                                      (`|SpawnActorFromClass` "/Game/Blueprint/BP_Bullet_Arrow_Reverse.BP_Bullet_Arrow_Reverse_C" (`KismetMathLibrary.MakeTransform` (260.0 -630.0 15.0)) "Undefined" "MultiplyWithRoot" null null))
                                                                                                                    (:`then_1`
                                                                                                                      (`KismetSystemLibrary.Delay` 0.2)
                                                                                                                      (`|SpawnActorFromClass` "/Game/Blueprint/BP_Bullet_Arrow_Reverse.BP_Bullet_Arrow_Reverse_C" (`KismetMathLibrary.MakeTransform` (-220.0 -630.0 15.0)) "Undefined" "MultiplyWithRoot" null null)
                                                                                                                      (`KismetSystemLibrary.Delay` 0.4)
                                                                                                                      (`|SpawnActorFromClass` "/Game/Blueprint/BP_Bullet_Arrow_Reverse.BP_Bullet_Arrow_Reverse_C" (`KismetMathLibrary.MakeTransform` (-180.0 -630.0 15.0)) "Undefined" "MultiplyWithRoot" null null)
                                                                                                                      (`KismetSystemLibrary.Delay` 0.4)
                                                                                                                      (`|SpawnActorFromClass` "/Game/Blueprint/BP_Bullet_Arrow_Reverse.BP_Bullet_Arrow_Reverse_C" (`KismetMathLibrary.MakeTransform` (-100.0 -630.0 15.0)) "Undefined" "MultiplyWithRoot" null null)
                                                                                                                      (`KismetSystemLibrary.Delay` 0.4)
                                                                                                                      (`|ExecutionSequence`
                                                                                                                        (:`then_0`
                                                                                                                          ;[1 1 1] Comment
                                                                                                                          (`|SpawnActorFromClass` "/Game/Blueprint/BP_Bullet_Pop.BP_Bullet_Pop_C" (`KismetMathLibrary.MakeTransform` (220.0 550.0 15.0)) "Undefined" "MultiplyWithRoot" null null)
                                                                                                                          (`KismetSystemLibrary.Delay` 2.4)
                                                                                                                          (`|SpawnActorFromClass` "/Game/Blueprint/BP_Bullet_Arrow.BP_Bullet_Arrow_C" (`KismetMathLibrary.MakeTransform` (-100.0 630.0 15.0)) "Undefined" "MultiplyWithRoot" null null)
                                                                                                                          (`KismetSystemLibrary.Delay` 0.4)
                                                                                                                          (`|ExecutionSequence`
                                                                                                                            (:`then_0`
                                                                                                                              (`KismetSystemLibrary.Delay` 0.2)
                                                                                                                              (`|SpawnActorFromClass` "/Game/Blueprint/BP_Bullet_Arrow.BP_Bullet_Arrow_C" (`KismetMathLibrary.MakeTransform` (200.0 630.0 15.0)) "Undefined" "MultiplyWithRoot" null null))
                                                                                                                            (:`then_1`
                                                                                                                              (`|SpawnActorFromClass` "/Game/Blueprint/BP_Bullet_Arrow.BP_Bullet_Arrow_C" (`KismetMathLibrary.MakeTransform` (-140.0 630.0 15.0)) "Undefined" "MultiplyWithRoot" null null)
                                                                                                                              (`KismetSystemLibrary.Delay` 0.4)
                                                                                                                              (`|ExecutionSequence`
                                                                                                                                (:`then_0`
                                                                                                                                  (`KismetSystemLibrary.Delay` 0.2)
                                                                                                                                  (`|SpawnActorFromClass` "/Game/Blueprint/BP_Bullet_Arrow.BP_Bullet_Arrow_C" (`KismetMathLibrary.MakeTransform` (-180.0 630.0 15.0)) "Undefined" "MultiplyWithRoot" null null)
                                                                                                                                  (`KismetSystemLibrary.Delay` 0.4)
                                                                                                                                  (`|SpawnActorFromClass` "/Game/Blueprint/BP_Bullet_Arrow.BP_Bullet_Arrow_C" (`KismetMathLibrary.MakeTransform` (-20.0 630.0 15.0)) "Undefined" "MultiplyWithRoot" null null)
                                                                                                                                  (`KismetSystemLibrary.Delay` 0.4)
                                                                                                                                  (`|SpawnActorFromClass` "/Game/Blueprint/BP_Bullet_Arrow.BP_Bullet_Arrow_C" (`KismetMathLibrary.MakeTransform` (-80.0 630.0 15.0)) "Undefined" "MultiplyWithRoot" null null)
                                                                                                                                  (`KismetSystemLibrary.Delay` 0.4)
                                                                                                                                  (`|SpawnActorFromClass` "/Game/Blueprint/BP_Bullet_Arrow.BP_Bullet_Arrow_C" (`KismetMathLibrary.MakeTransform` (260.0 630.0 15.0)) "Undefined" "MultiplyWithRoot" null null)
                                                                                                                                  (`KismetSystemLibrary.Delay` 0.4)
                                                                                                                                  (`|SpawnActorFromClass` "/Game/Blueprint/BP_Bullet_Arrow.BP_Bullet_Arrow_C" (`KismetMathLibrary.MakeTransform` (220.0 630.0 15.0)) "Undefined" "MultiplyWithRoot" null null)
                                                                                                                                  (`KismetSystemLibrary.Delay` 0.4)
                                                                                                                                  (`|SpawnActorFromClass` "/Game/Blueprint/BP_Bullet_Arrow.BP_Bullet_Arrow_C" (`KismetMathLibrary.MakeTransform` (0.0 630.0 15.0)) "Undefined" "MultiplyWithRoot" null null)
                                                                                                                                  (`|ExecutionSequence`
                                                                                                                                    (:`then_0`
                                                                                                                                      (`KismetSystemLibrary.Delay` 0.2)
                                                                                                                                      (`|SpawnActorFromClass` "/Game/Blueprint/BP_Bullet_Arrow.BP_Bullet_Arrow_C" (`KismetMathLibrary.MakeTransform` (200.0 630.0 15.0)) "Undefined" "MultiplyWithRoot" null null))
                                                                                                                                    (:`then_1`
                                                                                                                                      (`|SpawnActorFromClass` "/Game/Blueprint/BP_Bullet_Arrow.BP_Bullet_Arrow_C" (`KismetMathLibrary.MakeTransform` (-140.0 630.0 15.0)) "Undefined" "MultiplyWithRoot" null null)
                                                                                                                                      (`KismetSystemLibrary.Delay` 0.4)
                                                                                                                                      (`|ExecutionSequence`
                                                                                                                                        (:`then_0`
                                                                                                                                          (`KismetSystemLibrary.Delay` 0.2)
                                                                                                                                          (`|SpawnActorFromClass` "/Game/Blueprint/BP_Bullet_Arrow.BP_Bullet_Arrow_C" (`KismetMathLibrary.MakeTransform` (-180.0 630.0 15.0)) "Undefined" "MultiplyWithRoot" null null)
                                                                                                                                          (`KismetSystemLibrary.Delay` 0.4)
                                                                                                                                          (`|SpawnActorFromClass` "/Game/Blueprint/BP_Bullet_Arrow.BP_Bullet_Arrow_C" (`KismetMathLibrary.MakeTransform` (-20.0 630.0 15.0)) "Undefined" "MultiplyWithRoot" null null)
                                                                                                                                          (`KismetSystemLibrary.Delay` 0.4)
                                                                                                                                          (`|SpawnActorFromClass` "/Game/Blueprint/BP_Bullet_Arrow.BP_Bullet_Arrow_C" (`KismetMathLibrary.MakeTransform` (-80.0 630.0 15.0)) "Undefined" "MultiplyWithRoot" null null)
                                                                                                                                          (`KismetSystemLibrary.Delay` 0.4)
                                                                                                                                          (`|ExecutionSequence`
                                                                                                                                            (:`then_0`
                                                                                                                                              (`KismetSystemLibrary.Delay` 0.2)
                                                                                                                                              (`|SpawnActorFromClass` "/Game/Blueprint/BP_Bullet_Arrow.BP_Bullet_Arrow_C" (`KismetMathLibrary.MakeTransform` (200.0 630.0 15.0)) "Undefined" "MultiplyWithRoot" null null))
                                                                                                                                            (:`then_1`
                                                                                                                                              (`|SpawnActorFromClass` "/Game/Blueprint/BP_Bullet_Arrow.BP_Bullet_Arrow_C" (`KismetMathLibrary.MakeTransform` (-140.0 630.0 15.0)) "Undefined" "MultiplyWithRoot" null null)
                                                                                                                                              (`KismetSystemLibrary.Delay` 0.4)
                                                                                                                                              (`|ExecutionSequence`
                                                                                                                                                (:`then_0`
                                                                                                                                                  (`KismetSystemLibrary.Delay` 0.2)
                                                                                                                                                  (`|SpawnActorFromClass` "/Game/Blueprint/BP_Bullet_Arrow.BP_Bullet_Arrow_C" (`KismetMathLibrary.MakeTransform` (-180.0 630.0 15.0)) "Undefined" "MultiplyWithRoot" null null)
                                                                                                                                                  (`KismetSystemLibrary.Delay` 0.4)
                                                                                                                                                  (`|SpawnActorFromClass` "/Game/Blueprint/BP_Bullet_Arrow.BP_Bullet_Arrow_C" (`KismetMathLibrary.MakeTransform` (-20.0 630.0 15.0)) "Undefined" "MultiplyWithRoot" null null)
                                                                                                                                                  (`KismetSystemLibrary.Delay` 0.4)
                                                                                                                                                  (`|SpawnActorFromClass` "/Game/Blueprint/BP_Bullet_Arrow.BP_Bullet_Arrow_C" (`KismetMathLibrary.MakeTransform` (-80.0 630.0 15.0)) "Undefined" "MultiplyWithRoot" null null)
                                                                                                                                                  (`KismetSystemLibrary.Delay` 0.4)
                                                                                                                                                  ;[1 1 1] c
                                                                                                                                                  (`|ExecutionSequence`
                                                                                                                                                    (:`then_0`
                                                                                                                                                      (`self.K2_DestroyActor` _returnvalue_2))
                                                                                                                                                    (:`then_1`
                                                                                                                                                      (`self.K2_DestroyActor` (stale _returnvalue_13)))
                                                                                                                                                    (:`then_2`
                                                                                                                                                      (`self.K2_DestroyActor` (stale _returnvalue_14)))
                                                                                                                                                    (:`then_3`
                                                                                                                                                      (`self.K2_DestroyActor` _returnvalue))
                                                                                                                                                    (:`then_4`
                                                                                                                                                      (`self.K2_DestroyActor` _returnvalue_5))
                                                                                                                                                    (:`then_5`
                                                                                                                                                      (`self.K2_DestroyActor` (stale _returnvalue_11)))
                                                                                                                                                    (:`then_6`
                                                                                                                                                      (`self.K2_DestroyActor` _returnvalue_4))
                                                                                                                                                    (:`then_7`
                                                                                                                                                      (`self.K2_DestroyActor` (stale _returnvalue_12)))
                                                                                                                                                    (:`then_8`
                                                                                                                                                      (`self.K2_DestroyActor` _returnvalue_3))
                                                                                                                                                    (:`then_9`
                                                                                                                                                      (`self.K2_DestroyActor` _returnvalue_6))
                                                                                                                                                    (:`then_10`
                                                                                                                                                      (`self.K2_DestroyActor` _returnvalue_7))
                                                                                                                                                    (:`then_11`
                                                                                                                                                      (`self.K2_DestroyActor` (stale _returnvalue_9)))
                                                                                                                                                    (:`then_12`
                                                                                                                                                      (`self.K2_DestroyActor` _returnvalue_8))
                                                                                                                                                    (:`then_13`
                                                                                                                                                      (`self.K2_DestroyActor` (stale _returnvalue_10)))
                                                                                                                                                    (:`then_14`
                                                                                                                                                      (`KismetSystemLibrary.Delay` 4.0))))
                                                                                                                                                (:`then_1`
                                                                                                                                                  (`|SpawnActorFromClass` "/Game/Blueprint/BP_Bullet_Arrow.BP_Bullet_Arrow_C" (`KismetMathLibrary.MakeTransform` (-240.0 630.0 15.0)) "Undefined" "MultiplyWithRoot" null null))))))
                                                                                                                                        (:`then_1`
                                                                                                                                          (`|SpawnActorFromClass` "/Game/Blueprint/BP_Bullet_Arrow.BP_Bullet_Arrow_C" (`KismetMathLibrary.MakeTransform` (-240.0 630.0 15.0)) "Undefined" "MultiplyWithRoot" null null))))))
                                                                                                                                (:`then_1`
                                                                                                                                  (`|SpawnActorFromClass` "/Game/Blueprint/BP_Bullet_Arrow.BP_Bullet_Arrow_C" (`KismetMathLibrary.MakeTransform` (-240.0 630.0 15.0)) "Undefined" "MultiplyWithRoot" null null))))
                                                                                                                            (:`then_2`
                                                                                                                              (`|SpawnActorFromClass` "/Game/Blueprint/BP_Bullet_Arrow.BP_Bullet_Arrow_C" (`KismetMathLibrary.MakeTransform` (0.0 0.0 15.0)) "Undefined" "MultiplyWithRoot" null null))))
                                                                                                                        (:`then_1`
                                                                                                                          (`|SpawnActorFromClass` "/Game/Blueprint/BP_Bullet_Pop.BP_Bullet_Pop_C" (`KismetMathLibrary.MakeTransform` (110.0 550.0 15.0)) "Undefined" "MultiplyWithRoot" null null))
                                                                                                                        (:`then_2`
                                                                                                                          (`|SpawnActorFromClass` "/Game/Blueprint/BP_Bullet_Pop.BP_Bullet_Pop_C" (`KismetMathLibrary.MakeTransform` (0.0 550.0 15.0)) "Undefined" "MultiplyWithRoot" null null))
                                                                                                                        (:`then_3`
                                                                                                                          (`|SpawnActorFromClass` "/Game/Blueprint/BP_Bullet_Pop.BP_Bullet_Pop_C" (`KismetMathLibrary.MakeTransform` (-110.0 550.0 15.0)) "Undefined" "MultiplyWithRoot" null null))
                                                                                                                        (:`then_4`
                                                                                                                          (`|SpawnActorFromClass` "/Game/Blueprint/BP_Bullet_Pop.BP_Bullet_Pop_C" (`KismetMathLibrary.MakeTransform` (-220.0 550.0 15.0)) "Undefined" "MultiplyWithRoot" null null))))))))))))))))))))))
                                                                                (:`then_1`
                                                                                  (`|SpawnActorFromClass` "/Game/Blueprint/BP_Bullet_Arrow_Reverse.BP_Bullet_Arrow_Reverse_C" (`KismetMathLibrary.MakeTransform` (-240.0 -630.0 15.0)) "Undefined" "MultiplyWithRoot" null null))))
                                                                            (:`then_1`
                                                                              (`|SpawnActorFromClass` "/Game/Blueprint/BP_Bullet_Arrow_Reverse.BP_Bullet_Arrow_Reverse_C" (`KismetMathLibrary.MakeTransform` (-140.0 -630.0 15.0)) "Undefined" "MultiplyWithRoot" null null))
                                                                            (:`then_2`
                                                                              (`|SpawnActorFromClass` "/Game/Blueprint/BP_Bullet_Arrow_Reverse.BP_Bullet_Arrow_Reverse_C" (`KismetMathLibrary.MakeTransform` (0.0 0.0 15.0)) "Undefined" "MultiplyWithRoot" null null))))
                                                                        (:`then_1`
                                                                          (`|SpawnActorFromClass` "/Game/Blueprint/BP_Bullet_Pop_Reverse.BP_Bullet_Pop_Reverse_C" (`KismetMathLibrary.MakeTransform` (110.0 -240.0 15.0)) "Undefined" "MultiplyWithRoot" null null))
                                                                        (:`then_2`
                                                                          (`|SpawnActorFromClass` "/Game/Blueprint/BP_Bullet_Pop_Reverse.BP_Bullet_Pop_Reverse_C" (`KismetMathLibrary.MakeTransform` (0.0 -240.0 15.0)) "Undefined" "MultiplyWithRoot" null null))
                                                                        (:`then_3`
                                                                          (`|SpawnActorFromClass` "/Game/Blueprint/BP_Bullet_Pop_Reverse.BP_Bullet_Pop_Reverse_C" (`KismetMathLibrary.MakeTransform` (-110.0 -240.0 15.0)) "Undefined" "MultiplyWithRoot" null null))
                                                                        (:`then_4`
                                                                          (`|SpawnActorFromClass` "/Game/Blueprint/BP_Bullet_Pop_Reverse.BP_Bullet_Pop_Reverse_C" (`KismetMathLibrary.MakeTransform` (-220.0 -240.0 15.0)) "Undefined" "MultiplyWithRoot" null null))))
                                                                    (:`then_1`
                                                                      (`|SpawnActorFromClass` "/Game/Blueprint/BP_Bullet_Arrow.BP_Bullet_Arrow_C" (`KismetMathLibrary.MakeTransform` (-240.0 630.0 15.0)) "Undefined" "MultiplyWithRoot" null null))))
                                                                (:`then_2`
                                                                  (`|SpawnActorFromClass` "/Game/Blueprint/BP_Bullet_Arrow.BP_Bullet_Arrow_C" (`KismetMathLibrary.MakeTransform` (0.0 0.0 15.0)) "Undefined" "MultiplyWithRoot" null null))))
                                                            (:`then_1`
                                                              (`|SpawnActorFromClass` "/Game/Blueprint/BP_Bullet_Arrow.BP_Bullet_Arrow_C" (`KismetMathLibrary.MakeTransform` (-240.0 630.0 15.0)) "Undefined" "MultiplyWithRoot" null null))))
                                                        (:`then_2`
                                                          (`|SpawnActorFromClass` "/Game/Blueprint/BP_Bullet_Arrow.BP_Bullet_Arrow_C" (`KismetMathLibrary.MakeTransform` (0.0 0.0 15.0)) "Undefined" "MultiplyWithRoot" null null))))
                                                    (:`then_1`
                                                      (`|SpawnActorFromClass` "/Game/Blueprint/BP_Bullet_Arrow.BP_Bullet_Arrow_C" (`KismetMathLibrary.MakeTransform` (-240.0 630.0 15.0)) "Undefined" "MultiplyWithRoot" null null))))
                                                (:`then_2`
                                                  (`|SpawnActorFromClass` "/Game/Blueprint/BP_Bullet_Arrow.BP_Bullet_Arrow_C" (`KismetMathLibrary.MakeTransform` (0.0 0.0 15.0)) "Undefined" "MultiplyWithRoot" null null))))))
                                        (:`then_1`
                                          (`|SpawnActorFromClass` "/Game/Blueprint/BP_Bullet_Arrow.BP_Bullet_Arrow_C" (`KismetMathLibrary.MakeTransform` (-240.0 630.0 15.0)) "Undefined" "MultiplyWithRoot" null null))))
                                    (:`then_2`
                                      (`|SpawnActorFromClass` "/Game/Blueprint/BP_Bullet_Arrow.BP_Bullet_Arrow_C" (`KismetMathLibrary.MakeTransform` (0.0 0.0 15.0)) "Undefined" "MultiplyWithRoot" null null))))
                                (:`then_1`
                                  (`|SpawnActorFromClass` "/Game/Blueprint/BP_Bullet_Pop.BP_Bullet_Pop_C" (`KismetMathLibrary.MakeTransform` (110.0 550.0 15.0)) "Undefined" "MultiplyWithRoot" null null))
                                (:`then_2`
                                  (`|SpawnActorFromClass` "/Game/Blueprint/BP_Bullet_Pop.BP_Bullet_Pop_C" (`KismetMathLibrary.MakeTransform` (0.0 550.0 15.0)) "Undefined" "MultiplyWithRoot" null null))
                                (:`then_3`
                                  (`|SpawnActorFromClass` "/Game/Blueprint/BP_Bullet_Pop.BP_Bullet_Pop_C" (`KismetMathLibrary.MakeTransform` (-110.0 550.0 15.0)) "Undefined" "MultiplyWithRoot" null null))
                                (:`then_4`
                                  (`|SpawnActorFromClass` "/Game/Blueprint/BP_Bullet_Pop.BP_Bullet_Pop_C" (`KismetMathLibrary.MakeTransform` (-220.0 550.0 15.0)) "Undefined" "MultiplyWithRoot" null null))))
                            (:`then_1`
                              (bind _returnvalue_9 (`|SpawnActorFromClass` "/Game/Blueprint/BP_BUllet_BigCube.BP_BUllet_BigCube_C" (`KismetMathLibrary.MakeTransform` (85.0 325.0 15.0)) "Undefined" "MultiplyWithRoot" null null)))
                            (:`then_2`
                              (bind _returnvalue_10 (`|SpawnActorFromClass` "/Game/Blueprint/BP_BUllet_BigCube.BP_BUllet_BigCube_C" (`KismetMathLibrary.MakeTransform` (180.0 230.0 15.0)) "Undefined" "MultiplyWithRoot" null null)))))
                        (:`then_1`
                          (bind _returnvalue_11 (`|SpawnActorFromClass` "/Game/Blueprint/BP_BUllet_BigCube.BP_BUllet_BigCube_C" (`KismetMathLibrary.MakeTransform` (180.0 420.0 15.0)) "Undefined" "MultiplyWithRoot" null null)))))
                    (:`then_1`
                      (bind _returnvalue_12 (`|SpawnActorFromClass` "/Game/Blueprint/BP_BUllet_BigCube.BP_BUllet_BigCube_C" (`KismetMathLibrary.MakeTransform` (85.0 230.0 15.0)) "Undefined" "MultiplyWithRoot" null null)))))))
            (:`then_1`
              (bind _returnvalue_13 (`|SpawnActorFromClass` "/Game/Blueprint/BP_BUllet_BigCube.BP_BUllet_BigCube_C" (`KismetMathLibrary.MakeTransform` (200.0 -175.0 15.0)) "Undefined" "MultiplyWithRoot" null null)))
            (:`then_2`
              (bind _returnvalue_14 (`|SpawnActorFromClass` "/Game/Blueprint/BP_BUllet_BigCube.BP_BUllet_BigCube_C" (`KismetMathLibrary.MakeTransform` (240.0 120.0 15.0)) "Undefined" "MultiplyWithRoot" null null)))))
        (:`then_2`
          (`|SpawnActorFromClass` "/Game/Blueprint/BP_Bullet.BP_Bullet_C" (`KismetMathLibrary.MakeTransform` (120.0 480.0 15.0) (struct) (0.1 0.1 0.1)) "Undefined" "MultiplyWithRoot" null null))))
    (:`then_1`
      (`|SpawnActorFromClass` "/Game/Blueprint/BP_Bullet.BP_Bullet_C" (`KismetMathLibrary.MakeTransform` (-140.0 -200.0 15.0) (struct) (0.1 0.1 0.1)) "Undefined" "MultiplyWithRoot" null null)
      (goto _label))
    (:`then_2`
      (`|SpawnActorFromClass` "/Game/Blueprint/BP_Bullet.BP_Bullet_C" (`KismetMathLibrary.MakeTransform` (-220.0 -200.0 15.0) (struct) (0.1 0.1 0.1)) "Undefined" "MultiplyWithRoot" null null)
      (goto _label))
    (:`then_3`
      (`|SpawnActorFromClass` "/Game/Blueprint/BP_Bullet.BP_Bullet_C" (`KismetMathLibrary.MakeTransform` (-260.0 -40.0 15.0) (struct) (0.1 0.1 0.1)) "Undefined" "MultiplyWithRoot" null null)
      (goto _label))
    (:`then_4`
      (`|SpawnActorFromClass` "/Game/Blueprint/BP_Bullet.BP_Bullet_C" (`KismetMathLibrary.MakeTransform` (-220.0 80.0 15.0) (struct) (0.1 0.1 0.1)) "Undefined" "MultiplyWithRoot" null null))
    (:`then_5`
      (`|SpawnActorFromClass` "/Game/Blueprint/BP_Bullet.BP_Bullet_C" (`KismetMathLibrary.MakeTransform` (-260.0 160.0 15.0) (struct) (0.1 0.1 0.1)) "Undefined" "MultiplyWithRoot" null null))
    (:`then_6`
      (`|SpawnActorFromClass` "/Game/Blueprint/BP_Bullet.BP_Bullet_C" (`KismetMathLibrary.MakeTransform` (240.0 -140.0 15.0) (struct) (0.1 0.1 0.1)) "Undefined" "MultiplyWithRoot" null null))
    (:`then_7`
      (`|SpawnActorFromClass` "/Game/Blueprint/BP_Bullet.BP_Bullet_C" (`KismetMathLibrary.MakeTransform` (180.0 140.0 15.0) (struct) (0.1 0.1 0.1)) "Undefined" "MultiplyWithRoot" null null))
    (:`then_8`
      (`|SpawnActorFromClass` "/Game/Blueprint/BP_Bullet.BP_Bullet_C" (`KismetMathLibrary.MakeTransform` (140.0 300.0 15.0) (struct) (0.1 0.1 0.1)) "Undefined" "MultiplyWithRoot" null null))))

(fn `UserConstructionScript`)