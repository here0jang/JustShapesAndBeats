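; BP_Bullet1 is a bullet actor with a Cube component; its graphs handle only its lifetime.
; Tick accumulates elapsed time and destroys the actor after three seconds, so the six-second BeginPlay delay to destroy is effectively a fallback.
; Until then, Tick reapplies the current scale unchanged.
; SetBullet and the construction script are empty, and the material-parameter and zero-scale nodes are unconnected.
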(event `self.ReceiveBeginPlay`
  (`KismetSystemLibrary.Delay` 6.0)
  (`self.K2_DestroyActor`))

(event `self.ReceiveTick`
  (params (DeltaSeconds :type "Float (single-precision)"))
  (bind _output_get (set `self.CurrentTime` (+ DeltaSeconds (`self.CurrentTime`))))
  (if (> _output_get 3.0)
    (`self.K2_DestroyActor`)
    (else
      (`self.SetActorScale3D` (`self.GetActorScale3D`)))))

(fn `SetBullet`)

(fn `UserConstructionScript`)